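; A puzzle stand that accepts one prop_layer and marks itself solved when the layer's index matches its own.
; On box overlap it disables the layer's physics, snaps its transform, changes its collision responses, and swaps the hidden layer for a visible stand component.
; When a layer leaves a filled stand, it restores that layer's scale and visibility and empties the stand, but never clears Solved.
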(event OnComponentBeginOverlap(Box)
  (params (OtherActor :type Actor%20Object%20Reference) (OtherComp :type Primitive%20Component%20Object%20Reference) (OtherBodyIndex :type Integer) (bFromSweep :type Boolean) (SweepResult :type Hit%20Result%20Structure%20%28by%20ref%29))
  (if (not (Variables|Default|Getfilled))
    (bind _asprop_layer (Utilities|Casting|CastToprop_layer OtherActor))
    (|Locktostand _asprop_layer)
    (Variables|Default|Setfilled true)
    (Rendering|SetVisibility true false)
    (if (== (Variables|Default|GetlayerIndexStand) (Variables|/Game/Blueprints/prop_layer.prop_layer_C|GetLayerIndex _asprop_layer))
      (Variables|Default|Setsolved true))))

(event EventActorEndOverlap
  (params (OtherActor :type Actor%20Object%20Reference))
  (bind _asprop_layer (Utilities|Casting|CastToprop_layer OtherActor))
  (if (Variables|Default|Getfilled)
    (Default|SetScale _asprop_layer true (Variables|Default|GetlayerIndexStand))
    (Variables|Default|Setfilled false)
    (Collision|SetCollisionResponsetoChannel _asprop_layer "ECC_PhysicsBody" "ECR_Overlap")
    (Rendering|SetVisibility false false)
    (Rendering|SetVisibility _asprop_layer true false)))

(fn ConstructionScript)