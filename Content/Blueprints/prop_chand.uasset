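; Hanging prop Blueprint, apparently a chandelier, that swings with a decaying motion when StartSwing is called.
; A timeline track scaled by Swing drives relative pitch, and each completed pass cuts Swing by 10% and replays while it exceeds a small threshold.
; Every timeline update also clears sound mix modifiers, calls a reverb deactivation and plays a rope sound at the actor with tavern attenuation.
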(event Custom|StartSwing
  (bind _newtrack_0 (Timeline|Timeline_0 Play)
    (:Update
      (Transformation|SetRelativeRotation (Math|Rotator|MakeRotator (* _newtrack_0 (Variables|Default|GetSwing)) 0.0 0.0) false)
      (Class|GameplayStatics|ClearSoundMixModifiers)
      (Class|GameplayStatics|DeactivateReverbEffect "None")
      (Audio|PlaySoundatLocation "/Game/Audio/rope2.rope2" (Transformation|GetActorLocation) 1.0 1.0 0.0 "/Game/Audio/TavernSoundAtten.TavernSoundAtten"))
    (:Finished
      (Math|Float|CompareFloat (Variables|Default|GetSwing) 2.0
        (:>
          (bind _output_get (Variables|Default|SetSwing (* (stale _output_get) 0.9)))
          (Timeline|Timeline_0 PlayFromStart))
        (:<
          (Timeline|Timeline_0 Stop))))))

(fn ConstructionScript)