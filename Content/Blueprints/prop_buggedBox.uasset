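; Prop Blueprint for a "bugged box" that continuously oscillates its pCube2 morph target.
; The construction script seeds a random stream and draws a starting phase and a step size from it, so boxes vary in timing and speed.
; Tick passes through a short Delay to throttle updates, then advances the phase and feeds its degree-based sine into the morph weight.
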(event EventTick
  (params (DeltaSeconds :type Float%20%28single-precision%29))
  (Utilities|FlowControl|Delay 0.05)
  (bind _output_get (Variables|Default|SetrandomFloat (+ (stale _output_get) (Variables|Default|GetNewVar_0))))
  (Components|SkeletalMesh|SetMorphTarget "pCube2" (Math|Trig|Sin(Degrees) (Variables|Default|GetrandomFloat))))

(fn ConstructionScript
  (bind _stream (Variables|Default|Getstream))
  (bind _returnvalue (Math|Random|RandomFloatinRangefromStream 0.0 1e+01 _stream))
  (Class|KismetMathLibrary|SeedRandomStream (Variables|Default|Getstream))
  (Variables|Default|SetrandomFloat _returnvalue)
  (Variables|Default|SetNewVar_0 _returnvalue))