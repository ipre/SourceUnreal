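; Placeholder light prop Blueprint that can be switched on during play.
; The construction script sets visibility from the LightIsOn flag, so the starting state follows that variable.
; The Activate event, when the flag is off, plays a spotlight sound at the actor's location, turns visibility on and sets the flag.
; The graph has no switch-off path, so repeated activations do nothing.
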(event Custom|Activate
  ;[1 1 1] Activate
  (if (not (Variables|Default|GetLightIsOn))
    (Audio|PlaySoundatLocation "/Game/Audio/SpotLight/49023__reidmangan__spotlight-stereo.49023__reidmangan__spotlight-stereo" (Transformation|GetActorLocation))
    (Rendering|SetVisibility true false)
    (Variables|Default|SetLightIsOn true)))

(fn ConstructionScript
  (if (Variables|Default|GetLightIsOn)
    (Rendering|SetVisibility true false)
    (else
      (Rendering|SetVisibility false false))))