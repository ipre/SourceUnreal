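; Layered prop actor that blocks pawns and takes its material and, optionally, its size from a layer index.
; The construction script picks the material from the LayerMat array by LayerIndex, caches the world scale and sets Pawn collision to Block.
; SetScale either restores the default scale or derives a thin shape whose Y and Z scale grow with the layer index.
; BeginPlay calls it in default-scale mode.
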(event EventBeginPlay
  (CallFunction|SetScale true))

(fn ConstructionScript
  (Rendering|Material|SetMaterial 0 (Utilities|Array|Get(acopy) (Variables|Default|GetLayer_Mat) (Variables|Default|GetLayerIndex)))
  (Variables|Default|SetDefaultScale (Transformation|GetWorldScale))
  (Collision|SetCollisionResponsetoChannel "ECC_Pawn" "ECR_Block"))

(fn SetScale
  (params (DefaultScale :type Boolean :default false) (LayerIndex :type Integer :default 0))
  (bind _returnvalue (Math|Conversions|ToFloat(Integer) LayerIndex))
  (if DefaultScale
    (Transformation|SetActorScale3D (Variables|Default|GetDefaultScale))
    (else
      (Transformation|SetActorScale3D (* (Math|Vector|MakeVector 0.1 (+ (* 1.0 _returnvalue) 0.0) (+ 2.6 (* _returnvalue 0.5))) 1.3)))))