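; A floating prop that can be launched into a weightless, spinning drift and later dropped back down.
; The construction script sets the mesh from an array by index, seeds a random stream and derives a slow random rotation rate from it.
; Launch disables gravity, applies a random upward-biased impulse from that stream and activates RotatingMovement.
; BackToEarth restores gravity and switches all collision responses to overlap, so the prop falls without blocking.
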(event Custom|Launch
  (bind _stream (Variables|Default|Getstream))
  (Physics|SetEnableGravity false)
  (Physics|AddImpulse (Math|Vector|MakeVector (Math|Random|RandomFloatinRangefromStream -6e+03 6e+03 _stream) (Math|Random|RandomFloatinRangefromStream -6e+03 6e+03 _stream) (Math|Random|RandomFloatinRangefromStream 6e+03 3.2e+04 _stream)) "None" false)
  (Components|Activation|Activate (Variables|Default|GetRotatingMovement) false))

(event Custom|BackToEarth
  (Collision|SetCollisionResponsetoAllChannels "ECR_Overlap")
  (Physics|SetEnableGravity true))

(fn ConstructionScript
  (Components|StaticMesh|SetStaticMesh (Utilities|Array|Get(acopy) (Variables|Default|GetMeshArray) (Variables|Default|GetmeshIndex)))
  (Class|KismetMathLibrary|SeedRandomStream (Variables|Default|Getstream))
  (Variables|/Script/Engine.RotatingMovementComponent|SetRotationRate (Variables|Default|GetRotatingMovement) (* (Class|KismetMathLibrary|RandomRotatorfromStream true (Variables|Default|Getstream)) 0.1)))