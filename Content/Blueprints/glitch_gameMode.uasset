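; Game mode that respawns the player character after it is destroyed.
; On BeginPlay it casts player 0's pawn to char_player and binds to its OnDestroyed event.
; After a short delay, that event spawns a new char_player at the stored SpawnTransform and has the first player controller possess it.
; It then calls Respawn to rebind to the new character, so the cycle repeats.
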(event Custom|Respawn
  (bind _aschar_player (Utilities|Casting|CastTochar_player (Game|GetPlayerCharacter 0)))
  (Game|AssignOnDestroyed _aschar_player (delegate Custom|OnDestroyed_Event)))

(event Custom|OnDestroyed_Event
  (Utilities|FlowControl|Delay 1.0)
  (bind _returnvalue (Game|SpawnActorfromClass "/Game/Blueprints/char_player.char_player_C" (Variables|Default|GetSpawnTransform) false 0))
  (Pawn|Possess (Game|GetPlayerController 0) _returnvalue)
  (CallFunction|Respawn))

(event EventBeginPlay
  (bind _aschar_player (Utilities|Casting|CastTochar_player (Game|GetPlayerCharacter 0)))
  (Game|AssignOnDestroyed _aschar_player (delegate Custom|OnDestroyed_Event)))

(fn ConstructionScript)