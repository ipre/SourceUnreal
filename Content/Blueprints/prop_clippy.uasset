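; Clippy is a prop the player picks up and drops by interacting, which launches its holder off nearby surfaces.
; A FlipFlop attaches it to the first-person mesh's "clippy" socket or detaches it with physics restored.
; While held, a Tick-fed Gate runs a debug-drawn trace along its up vector.
; Hits launch the character along the impact normal, scaled by current speed, with a DoOnce and short delay as cooldown.
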(event Custom|Reset
  (Utilities|FlowControl|DoOnce false) ; enters at Reset
)

(event EventInteractwith
  (params (Player :type Char%20Player%20Object%20Reference))
  (bind _returnvalue (Transformation|GetActorLocation))
  (Utilities|FlowControl|FlipFlop
    (:A
      (bind _aschar_player (Utilities|Casting|CastTochar_player Player))
      (Physics|SetSimulatePhysics false)
      (Collision|SetCollisionResponsetoAllChannels "ECR_Block")
      (Collision|SetCollisionResponsetoChannel "ECC_Pawn" "ECR_Ignore")
      (Class|Actor|AttachRootComponentto (Variables|/Game/Blueprints/char_player.char_player_C|GetMesh1P _aschar_player) "clippy" "SnapToTarget" true)
      (Rendering|SetVisibility (Variables|Default|GetTextRender) false false)
      (Utilities|FlowControl|Gate true) ; enters at Open
    )
    (:B
      (Class|SceneComponent|DetachfromParent true)
      (Collision|SetCollisionResponsetoChannel "ECC_Pawn" "ECR_Block")
      (Physics|SetSimulatePhysics true)
      (Utilities|FlowControl|Gate true) ; enters at Close
    )))

(event EventTick
  (params (DeltaSeconds :type Float%20%28single-precision%29))
  (bind _returnvalue (Transformation|GetActorLocation))
  (Utilities|FlowControl|Gate true
    (:Exit
      (bind (_outhit _returnvalue_2) (Collision|LineTraceForObjects _returnvalue (+ _returnvalue (* (Math|Vector|GetUpVector (Transformation|GetActorRotation)) 2e+02)) (Variables|Default|GetObjectType) true 0 "ForOneFrame"))
      (if _returnvalue_2
        (Utilities|FlowControl|DoOnce false
          (:Completed
            (Character|LaunchCharacter (stale EventInteractwith _aschar_player) (Math|Vector|MakeVector (* (Class|KismetMathLibrary|MapRange (Math|Vector2D|Vector2DLength (Math|Vector2D|MakeVector2D (.X (Math|Vector|BreakVector (Transformation|GetVelocity (stale EventInteractwith _aschar_player)))) (.Y (Math|Vector|BreakVector (Transformation|GetVelocity (stale EventInteractwith _aschar_player)))))) 0.0 6e+02 3e+02 7e+02) (.X (Math|Vector|BreakVector (.ImpactNormal (Collision|BreakHitResult _outhit)))) 1.5) (* (.Y (Math|Vector|BreakVector (.ImpactNormal (Collision|BreakHitResult _outhit)))) (Class|KismetMathLibrary|MapRange (Math|Vector2D|Vector2DLength (Math|Vector2D|MakeVector2D (.X (Math|Vector|BreakVector (Transformation|GetVelocity (stale EventInteractwith _aschar_player)))) (.Y (Math|Vector|BreakVector (Transformation|GetVelocity (stale EventInteractwith _aschar_player)))))) 0.0 6e+02 3e+02 7e+02) 1.5) (* (.Z (Math|Vector|BreakVector (.ImpactNormal (Collision|BreakHitResult _outhit)))) (Math|Float|Clamp(Float) (* -1.0 (.Z (Math|Vector|BreakVector (Transformation|GetVelocity (stale EventInteractwith _aschar_player))))) 5e+02 5e+03))) false true)
            (Utilities|FlowControl|Delay 0.1)
            (CallFunction|Reset)))))))

(fn ConstructionScript)