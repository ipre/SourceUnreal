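; Construction-script Blueprint that builds a wall by tiling a chosen mesh as instances on the Wall component.
; The X and Z extents of a size vector, divided by the tile dimensions and floored, set the loop bounds for a vertical grid spaced by those dimensions.
; An optional flag replaces the mesh's first material slot with a custom material.
; The event graph holds only empty events.
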(event EventBeginPlay)

(event EventActorBeginOverlap
  (params (OtherActor :type Actor%20Object%20Reference)))

(event EventTick
  (params (DeltaSeconds :type Float%20%28single-precision%29)))

(fn ConstructionScript
  (bind _wall (Variables|Default|Getwall))
  (bind _vector (Variables|Default|GetVector))
  (Utilities|FlowControl|Sequence
    (:then_0
      (Components|StaticMesh|SetStaticMesh _wall (Variables|Default|GetMesh))
      (for _index (range 0 (Math|Float|Floor (/ (.x _vector) (Math|Conversions|ToFloat(Integer) (Variables|Default|GetDimensionX)))))
        (for _index_2 (range 0 (Math|Float|Floor (/ (.z _vector) (Math|Conversions|ToFloat(Integer) (Variables|Default|GetDimensionY)))))
          (Components|InstancedStaticMesh|AddInstance (Math|Transform|MakeTransform (Math|Vector|MakeVector (Math|Conversions|ToFloat(Integer) (* _index (Variables|Default|GetDimensionX))) 0.0 (Math|Conversions|ToFloat(Integer) (* _index_2 (Variables|Default|GetDimensionY)))) "0, 0, 0" "1,1,1")))))
    (:then_1
      (if (Variables|Default|GetchangeMaterial)
        (Rendering|Material|SetMaterial _wall 0 (Variables|Default|GetCustomMat))))))