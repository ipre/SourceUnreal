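; A prop Blueprint that launches the player character skyward when an actor overlaps it, unless IsDisabled is set.
; On overlap it prints a debug string and calls LaunchCharacter on player 0 with a fixed, mostly upward velocity, whichever actor triggered it.
; The cast to char_player is disconnected, and a facing-based knockback calculation using KnockbackPower is left unused.
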(event EventActorBeginOverlap
  (params (OtherActor :type Actor%20Object%20Reference))
  (if (not (Variables|Default|GetisDisabled))
    (Development|PrintString "get_rekt")
    (Character|LaunchCharacter (Game|GetPlayerCharacter 0) "0,1000.000000,10000.000000" false false)))

(fn ConstructionScript)