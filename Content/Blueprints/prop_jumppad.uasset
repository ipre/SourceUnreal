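; Jump pad prop that launches the player upward when something begins overlapping its Box.
; If JumpActive is set and no cooldown is running, the overlap adds LaunchPower to player character 0's vertical velocity, whichever actor triggered it.
; A latent Delay holds IsOnCooldown for a short period before re-arming the pad, with debug prints marking both state changes.
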(event OnComponentBeginOverlap(Box)
  (params (OtherActor :type Actor%20Object%20Reference) (OtherComp :type Primitive%20Component%20Object%20Reference) (OtherBodyIndex :type Integer) (bFromSweep :type Boolean) (SweepResult :type Hit%20Result%20Structure%20%28by%20ref%29))
  (if (Variables|Default|GetJumpActive)
    (if (not (Variables|Default|GetisOnCooldown))
      (Character|LaunchCharacter (Game|GetPlayerCharacter 0) (Math|Vector|MakeVector 0.0 0.0 (Variables|Default|GetLaunch%20power)) false false)
      (Variables|Default|SetisOnCooldown true)
      (Development|PrintString "jump is on cd")
      (Utilities|FlowControl|Delay 2.0)
      (Variables|Default|SetisOnCooldown false)
      (Development|PrintString "jump is ready"))))

(fn ConstructionScript)