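; A puzzle stand that snaps an overlapping puppet into place and checks whether it is the right one.
; The first puppet is repositioned, stops simulating physics, blocks pawns, and sets Solved if its pose index matches KeyIndex.
; A Check flag prevents repeat placement until a puppet leaves the Box.
; An overlapping NPC instead switches to a single animation and marks the stand solved without a key check.
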(event OnComponentEndOverlap(Box)
  (params (OtherActor :type Actor%20Object%20Reference) (OtherComp :type Primitive%20Component%20Object%20Reference) (OtherBodyIndex :type Integer))
  ;[1 1 1] checks for right puppet
  (Utilities|Casting|CastToprop_puppet OtherActor)
  (Variables|Default|Setcheck false))

(event EventActorBeginOverlap
  (params (OtherActor :type Actor%20Object%20Reference))
  ;[1 1 1] checks for right puppet
  (bind _asprop_puppet (Utilities|Casting|CastToprop_puppet OtherActor)
    (:then
      (if (not (Variables|Default|Getcheck))
        (Variables|Default|Setcheck true)
        (Transformation|SetWorldLocationAndRotation _asprop_puppet (Utilities|NewPuppetLocation) (Transformation|GetActorRotation) false)
        (Physics|SetSimulatePhysics _asprop_puppet false)
        (Collision|SetCollisionResponsetoChannel _asprop_puppet "ECC_Pawn" "ECR_Block")
        (if (== (Variables|/Game/Blueprints/prop_puppet.prop_puppet_C|Getposeindex _asprop_puppet) (Variables|Default|GetkeyIndex))
          (Variables|Default|Setsolved true))))
    (:CastFailed
      (bind _aschar_npc (Utilities|Casting|CastTochar_npc OtherActor))
      (Components|Animation|SetAnimationMode _aschar_npc "AnimationSingleNode")
      (Components|Animation|SetAnimation _aschar_npc "/Game/ThirdPersonBP/Character/ThirdPersonSkeleton_Sequence3.ThirdPersonSkeleton_Sequence3")
      (Transformation|SetWorldLocationAndRotation (Utilities|NewPuppetLocation) (Transformation|GetActorRotation) false)
      (Variables|Default|Setsolved true))))

(fn ConstructionScript)