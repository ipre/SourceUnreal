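; Shelf-row prop Blueprint that procedurally builds grids of shelves from a single instanced static mesh component.
; The construction script runs four nested loops over units, stack height, row count and shelves per row, adding one instance at each fixed-spacing grid point.
; Rows repeat along X, shelves and units along Y with extra per-unit Displacement, and levels stack in Z.
; An unconnected MultiGate remains from a random-shelf option and never runs.
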(fn ConstructionScript
  (for _index (range 0 (- (Variables|Default|GetUnits) 1))
    (for _index_2 (range 0 (- (Variables|Default|GetrowHeight) 1))
      (for _index_3 (range 0 (- (Variables|Default|GetRowNumber) 1))
        (for _index_4 (range 0 (- (Variables|Default|GetShelfsInRows) 1))
          (Components|InstancedStaticMesh|AddInstance (Variables|Default|GetInstancedStaticMesh) (Math|Transform|MakeTransform (Math|Vector|MakeVector (* _index_3 7e+02) (+ (* _index_4 3e+02) (* _index 5e+02) (* _index (Variables|Default|Getdisplacement))) (* _index_2 3.4e+02)) "0, 0, 0" "1,1,1")))))))