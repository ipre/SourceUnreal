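; Interactive door prop that toggles open and closed through a FlipFlop on Interactwith.
; The Open_door timeline plays or reverses, setting yaw from its curve times a direction, offset by the actor yaw cached in the construction script.
; CalculateDoorDirection's player-facing dot-product nodes are unused, and the box overlap only reaches a DoOnce gated by Canopen, with nothing after it.
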(event OnComponentBeginOverlap(Box)
  (params (OtherActor :type Actor%20Object%20Reference) (OtherComp :type Primitive%20Component%20Object%20Reference) (OtherBodyIndex :type Integer) (bFromSweep :type Boolean) (SweepResult :type Hit%20Result%20Structure%20%28by%20ref%29))
  (if (Variables|Default|Getcanopen)
    (Utilities|FlowControl|DoOnce false)))

(event EventInteractwith
  (Utilities|FlowControl|FlipFlop
    (:A
      (Variables|Default|SetDoorDirection (Utilities|CalculateDoorDirection))
      (bind _doorrotation (Timeline|open_door Play)
        (:Update
          (Transformation|SetRelativeRotation (Math|Rotator|MakeRotator 0.0 (+ (* _doorrotation (Variables|Default|GetDoorDirection)) (Variables|Default|GetDoorRotation)) 0.0) false))))
    (:B
      (Timeline|open_door Reverse))))

(fn ConstructionScript
  (Variables|Default|SetDoorRotation (.Yaw (Class|KismetMathLibrary|BreakRot (Transformation|GetActorRotation)))))