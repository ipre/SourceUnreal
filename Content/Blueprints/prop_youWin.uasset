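; prop_youWin is a win-condition prop that appears once every puzzle trigger in its array is solved.
; On Tick, after a 0.2-second delay, it recounts the solved entries with a counter helper.
; When the count equals the array length, it makes a component visible and calls CallWinningCond to signal the win.
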(event EventTick
  (params (DeltaSeconds :type Float%20%28single-precision%29))
  (bind _array (Variables|Default|GetArray))
  ;[1 1 1] Check if all triggers are solved
  (Utilities|FlowControl|Delay 0.2)
  (Variables|Default|Setcheck 0)
  (for (_ _array_index) _array
    (if (Variables|/Game/Blueprints/prop_puzzle_gap.prop_puzzle_gap_C|Getsolved (Utilities|Array|Get(acopy) (Variables|Default|GetArray) _array_index))
      (CallFunction|Check++)))
  (if (== (Utilities|Array|Length _array) (Variables|Default|Getcheck))
    (Rendering|SetVisibility true false)
    (Default|CallWinningCond)))

(fn ConstructionScript)

(fn Check++
  (bind _output_get (Variables|Default|Setcheck (+ (stale _output_get) 1)))
  (return))