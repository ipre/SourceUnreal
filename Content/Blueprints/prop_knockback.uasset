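; Knockback prop that launches an overlapping char_player along the prop's forward vector, scaled by KnockbackPower.
; On overlap, if enabled, it disables player movement, waits briefly, switches to Flying mode and calls LaunchCharacter.
; Tick enables it only while the dot of player forward and the unnormalized offset to the prop exceeds a threshold, so distance affects this facing check.
; Walking mode is not restored here.
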(event EventActorBeginOverlap
  (params (OtherActor :type Actor%20Object%20Reference))
  (bind _returnvalue (Transformation|GetActorForwardVector))
  (bind (_x _y _z) (Math|Vector|BreakVector _returnvalue))
  ;[1 1 1] Knockback on overlap
  (bind _aschar_player (Utilities|Casting|CastTochar_player OtherActor))
  (if (not (Variables|Default|GetisDisabled))
    (Pawn|Components|CharacterMovement|DisableMovement _aschar_player)
    (Utilities|FlowControl|Delay 0.2)
    (Pawn|Components|CharacterMovement|SetMovementMode _aschar_player "MOVE_Flying" 0)
    (Character|LaunchCharacter _aschar_player (* (Math|Vector|MakeVector _x _y _z) (Variables|Default|GetKnockbackPower)) false false)))

(event EventTick
  (params (DeltaSeconds :type Float%20%28single-precision%29))
  (bind _returnvalue (Game|GetPlayerCharacter 0))
  (Variables|Default|SetisDisabled (not (> (Math|Vector|DotProduct (Transformation|GetActorForwardVector _returnvalue) (- (Transformation|GetActorLocation) (Transformation|GetActorLocation _returnvalue))) 0.9))))

(fn ConstructionScript)