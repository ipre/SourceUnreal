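; Level cube actor that slides its static mesh along an offset, with scale set in the construction script.
; On BeginPlay it can randomize speed and per-axis scale, then starts a timeline if movement is enabled.
; The timeline lerps the mesh's relative location from the stored actor position by the end offset.
; When finished it either resets and restarts through LoopingMove or destroys the actor.
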(event Custom|LoopingMove
  (bind _newtrack_3 (Timeline|Timeline_0 PlayFromStart)
    (:Update
      (Transformation|SetRelativeLocation (Variables|Debug|GetStaticMeshComponent) (Math|Vector|Lerp(Vector) (stale EventBeginPlay _output_get) (+ (stale EventBeginPlay _output_get) (Variables|Default|GetEndPos2)) _newtrack_3) false))
    (:Finished
      (if (Variables|Default|Getloop)
        (Transformation|SetRelativeLocation (Variables|Debug|GetStaticMeshComponent) (Variables|Default|GetActorPos) false)
        (CallFunction|LoopingMove)
        (else
          (Actor|DestroyActor))))))

(event EventBeginPlay
  (bind _returnvalue (Math|Random|RandomFloatinRange 0.5 1.4))
  (Variables|Default|SetEndPos2 (Variables|Default|GetEndPos))
  (if (Variables|Default|Getrandomize)
    (Variables|Default|Setspeed (Math|Random|RandomFloatinRange 0.3 1.3))
    (Transformation|SetRelativeScale3D (Variables|Debug|GetStaticMeshComponent) (Math|Vector|MakeVector _returnvalue _returnvalue _returnvalue)))
  (if (Variables|Default|Getmove)
    (bind _output_get (Variables|Default|SetActorPos (Transformation|GetActorLocation)))
    (Components|Timeline|SetPlayRate (Variables|Default|Getspeed))
    (bind _newtrack_3 (Timeline|Timeline_0 Play)
      (:Update
        (Transformation|SetRelativeLocation (Variables|Debug|GetStaticMeshComponent) (Math|Vector|Lerp(Vector) _output_get (+ _output_get (Variables|Default|GetEndPos2)) _newtrack_3) false))
      (:Finished
        (if (Variables|Default|Getloop)
          (Transformation|SetRelativeLocation (Variables|Debug|GetStaticMeshComponent) (Variables|Default|GetActorPos) false)
          (CallFunction|LoopingMove)
          (else
            (Actor|DestroyActor)))))))

(fn ConstructionScript
  (Transformation|SetWorldScale3D (Variables|Debug|GetStaticMeshComponent) (Variables|Default|GetCubeScale)))