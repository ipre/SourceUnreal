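; NPC character that registers itself on the GlitchGameInstance, turns toward the player and can follow them.
; Tick drives both behaviors through gates: LookAt overlap enables smoothed turning while nearly stationary, and Interactwith toggles following.
; Following uses simple AI moves and stops within close range, while a Box overlap sets OnHead.
; Path movement is an unfinished stub, and RotFromNpcToPlayer contains only unused nodes.
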(event OnComponentBeginOverlap(LookAt)
  (params (OtherActor :type Actor%20Object%20Reference) (OtherComp :type Primitive%20Component%20Object%20Reference) (OtherBodyIndex :type Integer) (bFromSweep :type Boolean) (SweepResult :type Hit%20Result%20Structure%20%28by%20ref%29))
  ;[0.4785 0.9618 1] LookAtPlayer
  (Utilities|Casting|CastTochar_player OtherActor)
  (Utilities|FlowControl|Gate true) ; enters at Open
)

(event OnComponentEndOverlap(LookAt)
  (params (OtherActor :type Actor%20Object%20Reference) (OtherComp :type Primitive%20Component%20Object%20Reference) (OtherBodyIndex :type Integer))
  ;[0.4785 0.9618 1] LookAtPlayer
  (Utilities|Casting|CastTochar_player OtherActor)
  (Utilities|FlowControl|Gate true) ; enters at Close
)

(event OnComponentBeginOverlap(Box)
  (params (OtherActor :type Actor%20Object%20Reference) (OtherComp :type Primitive%20Component%20Object%20Reference) (OtherBodyIndex :type Integer) (bFromSweep :type Boolean) (SweepResult :type Hit%20Result%20Structure%20%28by%20ref%29))
  ;[1 1 1] for prePub
  (Utilities|Casting|CastTochar_player OtherActor)
  (Variables|Default|SetOnHead true))

(event OnComponentEndOverlap(Box)
  (params (OtherActor :type Actor%20Object%20Reference) (OtherComp :type Primitive%20Component%20Object%20Reference) (OtherBodyIndex :type Integer))
  ;[1 1 1] for prePub
  (Utilities|Casting|CastTochar_player OtherActor)
  (Variables|Default|SetOnHead false))

(event Custom|MoveAlongPath
  ;[1 1 1] MoveAlongPath-wip
  (if (Variables|Default|GetFreeWalk)
    _))

(event Custom|LookAtPlayer
  ;[0.4785 0.9618 1] LookAtPlayer
  (if (Variables|Default|GetshouldLookAt)
    (Utilities|FlowControl|Gate true
      (:Exit
        (Math|Float|CompareFloat (Math|Vector|VectorLength (Transformation|GetVelocity)) 1e+01
          (:<
            (Transformation|SetActorRotation (Math|Interpolation|RInterpTo (Transformation|GetActorRotation) (Utilities|RotfromNpctoPlayer) (Variables|Default|GetdeltaTime) 5.0))))))))

(event Custom|StopFollow
  ;[1 1 1] Follow
  (Utilities|FlowControl|Gate true) ; enters at Close
)

(event Custom|FollowPlayer
  ;[1 1 1] Follow
  (if (Variables|Movement|Getfollow)
    (Utilities|FlowControl|Gate true
      (:Exit
        (if (< 1.5e+02 (Transformation|GetDistanceTo (Game|GetPlayerCharacter 0)))
          (AI|Navigation|SimpleMovetoLocation (Pawn|GetController) (Transformation|GetActorLocation (Game|GetPlayerCharacter 0)))
          (else
            (Components|Movement|StopMovementImmediately (Variables|Character|GetCharacterMovement))))))))

(event EventBeginPlay
  (bind _asglitch_game_instance (Utilities|Casting|CastToGlitchGameInstance (Game|GetGameInstance)))
  (bind _output_get (Variables|/Game/Blueprints/GlitchGameInstance.GlitchGameInstance_C|SetNPCChar _asglitch_game_instance self))
  (Development|PrintString (Utilities|GetDisplayName _output_get)))

(event EventTick
  (params (DeltaSeconds :type Float%20%28single-precision%29))
  ;[1 1 1] EventTick
  (Variables|Default|SetdeltaTime DeltaSeconds)
  (if (Variables|Default|GetcanMove)
    (CallFunction|LookatPlayer)
    (if (Variables|Default|GetFreeWalk)
      (CallFunction|FollowPlayer))))

(event EventInteractwith
  (params (Player :type Char%20Player%20Object%20Reference))
  ;[1 1 1] Follow
  (Utilities|FlowControl|Gate true) ; enters at Toggle
)

(fn ConstructionScript)