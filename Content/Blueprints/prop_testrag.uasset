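; A test ragdoll prop that toggles physics simulation when hit by a first-person projectile.
; A FlipFlop alternates between turning simulation on and turning it off on the skeletal mesh, then snapping the actor to a fixed rotation.
; Follow logic that would move toward the player pawn is present but never runs.
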(event EventHit
  (params (MyComp :type Primitive%20Component%20Object%20Reference) (Other :type Actor%20Object%20Reference) (OtherComp :type Primitive%20Component%20Object%20Reference) (bSelfMoved :type Boolean) (HitLocation :type Vector :default "0, 0, 0") (HitNormal :type Vector :default "0, 0, 0") (NormalImpulse :type Vector :default "0, 0, 0") (Hit :type Hit%20Result%20Structure%20%28by%20ref%29))
  ;[1 1 1] ragdoll
  (Utilities|Casting|CastToFirstPersonProjectile Other)
  (Utilities|FlowControl|FlipFlop
    (:A
      (Physics|SetSimulatePhysics true))
    (:B
      (Physics|SetSimulatePhysics (Variables|SkeletalMeshActor|GetSkeletalMeshComponent) false)
      (Transformation|SetActorRotation "0, 0,90.000000"))))

(fn ConstructionScript)