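; Physics cube prop, by its name, that shows its CubeIndex on front and back text components.
; The construction script sets both texts and makes the mesh block the Pawn channel.
; HighlightOnDistance toggles custom depth at a hardcoded 500 units from the player, using Distance only for its return value, which is false when nearer.
; That function's only call is in unconnected event-graph nodes, and Tick is empty, so highlighting never runs here.
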(event EventTick
  (params (DeltaSeconds :type Float%20%28single-precision%29)))

(fn ConstructionScript
  (Collision|SetCollisionResponsetoChannel (Variables|Debug|GetStaticMeshComponent) "ECC_Pawn" "ECR_Block")
  (Rendering|Components|TextRender|SetText (Variables|Default|GetfrontText) (Utilities|String|ToString(Integer) (Variables|Default|GetcubeIndex))))

(fn HighlightonDistance
  (params (StaticMeshComponent :type Static%20Mesh%20Component%20Object%20Reference) (Distance :type Float%20%28single-precision%29))
  (bind _returnvalue (Game|GetPlayerCharacter 0))
  (bind _returnvalue_2 (Transformation|GetDistanceTo _returnvalue))
  (Math|Float|CompareFloat _returnvalue_2 5e+02
    (:>
      (Rendering|SetRenderCustomDepth StaticMeshComponent false))
    (:<
      (Rendering|SetRenderCustomDepth StaticMeshComponent true)))
  (return (select (< _returnvalue_2 Distance) false true)))