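; A puzzle socket prop that accepts a physics cube whose CubeIndex matches its HoleIndex.
; A matching overlap turns the light green, sets Solved, then locks the cube at a fixed offset by disabling physics and making it WorldStatic.
; While unsolved, wrong cubes briefly freeze, then resume physics as the light turns red.
; A looping WrongObject timer blinks visibility until the overlap ends or the socket is solved.
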(event OnComponentBeginOverlap(Box)
  (params (OtherActor :type Actor%20Object%20Reference) (OtherComp :type Primitive%20Component%20Object%20Reference) (OtherBodyIndex :type Integer) (bFromSweep :type Boolean) (SweepResult :type Hit%20Result%20Structure%20%28by%20ref%29))
  (bind _returnvalue (Transformation|GetActorLocation))
  ;[1 1 1] Comment
  (bind _asprop_physics_cube (Utilities|Casting|CastToprop_physicsCube OtherActor)
    (:then
      (if (== (Variables|Default|GetholeIndex) (Variables|/Game/Blueprints/prop_physicsCube.prop_physicsCube_C|GetcubeIndex _asprop_physics_cube))
        (Rendering|SetVisibility false false)
        (Rendering|SetVisibility true false)
        (Rendering|Components|Light|SetLightColor "(R=0.077775,G=0.915000,B=0.168495,A=1.000000)")
        (Rendering|SetVisibility true false)
        (Variables|Default|Setsolved true)
        (Utilities|FlowControl|Delay 0.1)
        (Physics|SetSimulatePhysics (Variables|/Script/Engine.StaticMeshActor|GetStaticMeshComponent _asprop_physics_cube) false)
        (Transformation|SetActorLocationAndRotation _asprop_physics_cube (Math|Vector|MakeVector (- (.x _returnvalue) -4e+01) (- (.y _returnvalue) -3e+01) (+ (.z _returnvalue) 7e+01)) "180.000000, 0, 0")
        (Utilities|Time|ClearTimerbyFunctionName 0 "WrongObject")
        (Collision|SetCollisionObjectType (Variables|/Script/Engine.StaticMeshActor|GetStaticMeshComponent _asprop_physics_cube) "ECC_WorldStatic")
        (else
          (if (not (Variables|Default|Getsolved)) :!label _label
            (Utilities|FlowControl|Delay 0.1)
            (Physics|SetSimulatePhysics (Variables|/Script/Engine.StaticMeshActor|GetStaticMeshComponent _asprop_physics_cube) false)
            (Utilities|FlowControl|Delay 0.2)
            (Physics|SetSimulatePhysics (Variables|/Script/Engine.StaticMeshActor|GetStaticMeshComponent _asprop_physics_cube) true)
            (Rendering|Components|Light|SetLightColor "(R=0.915000,G=0.116508,B=0.081546,A=1.000000)")
            (Utilities|Time|SetTimerbyEvent (delegate Custom|WrongObject) 1.0 true)))))
    (:CastFailed
      (goto _label))))

(event Custom|WrongObject
  ;[1 1 1] Comment
  (Rendering|SetVisibility true false)
  (Rendering|SetVisibility true false)
  (Utilities|FlowControl|RetriggerableDelay 0.5)
  (Rendering|SetVisibility false false)
  (Rendering|SetVisibility false false))

(event EventActorEndOverlap
  (params (OtherActor :type Actor%20Object%20Reference))
  ;[1 1 1] Comment
  (Utilities|Time|ClearTimerbyFunctionName 0 "WrongObject"))

(fn ConstructionScript)